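; BP_CameraCharacter is a Character that serves as a movable camera rig with pan, orbit, pitch and zoom controls.
; It starts at a fixed world location with a long spring arm.
; Its events move it along spring arm axes, orbit via controller yaw, clamp arm pitch and zoom by changing arm length without limits.
; MovementComponent supplies the speeds and pitch limits.
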(event Custom|CameraOrbit
  (params (Magnitude :type Float%20%28double-precision%29))
  (Pawn|Input|AddControllerYawInput (* Magnitude (Variables|/Game/CameraMovementComponent.CameraMovementComponent_C|GetOrbitSpeed (Variables|Default|GetMovementComponent)))))

(event Custom|CameraForwardBackward
  (params (Magnitude :type Float%20%28double-precision%29))
  (Pawn|Input|AddMovementInput (Math|Vector|GetForwardVector (Variables|Default|GetSpringArm)) (* Magnitude (Variables|/Game/CameraMovementComponent.CameraMovementComponent_C|GetMoveSpeed (Variables|Default|GetMovementComponent))) false))

(event Custom|CameraLeftRight
  (params (Movement :type Float%20%28double-precision%29))
  (Pawn|Input|AddMovementInput (Math|Vector|GetRightVector (Variables|Default|GetSpringArm)) (* Movement (Variables|/Game/CameraMovementComponent.CameraMovementComponent_C|GetMoveSpeed (Variables|Default|GetMovementComponent))) false))

(event Custom|CameraPitch
  (params (Magnitude :type Float%20%28double-precision%29))
  (bind _springarm (Variables|Default|GetSpringArm))
  (bind _movementcomponent (Variables|Default|GetMovementComponent))
  (bind _returnvalue (Transformation|GetWorldRotation _springarm))
  (bind (_roll _pitch _yaw) (Math|Rotator|BreakRotator _returnvalue))
  (Transformation|SetWorldRotation (Variables|Default|GetSpringArm) (Math|Conversions|RotationFromXVector (Math|Rotator|GetRotationXVector (Math|Rotator|MakeRotator _roll (Math|Float|ClampAngle (+ (* (Variables|/Game/CameraMovementComponent.CameraMovementComponent_C|GetOrbitSpeed (Variables|Default|GetMovementComponent)) Magnitude) _pitch) (Variables|/Game/CameraMovementComponent.CameraMovementComponent_C|GetClampAngleMin _movementcomponent) (Variables|/Game/CameraMovementComponent.CameraMovementComponent_C|GetClampAngleMax _movementcomponent)) _yaw))) false false))

(event Custom|CameraZoomIn
  (params (Magnitude :type Float%20%28double-precision%29))
  (bind _springarm (Variables|Default|GetSpringArm))
  (Variables|/Script/Engine.SpringArmComponent|SetTargetArmLength _springarm (- (Variables|/Script/Engine.SpringArmComponent|GetTargetArmLength _springarm) (* Magnitude (Variables|/Game/CameraMovementComponent.CameraMovementComponent_C|GetZoomSpeed (Variables|Default|GetMovementComponent))))))

(event Custom|CameraZoomOut
  (params (Magnitude :type Float%20%28double-precision%29))
  (bind _springarm (Variables|Default|GetSpringArm))
  (Variables|/Script/Engine.SpringArmComponent|SetTargetArmLength _springarm (+ (Variables|/Script/Engine.SpringArmComponent|GetTargetArmLength _springarm) (* Magnitude (Variables|/Game/CameraMovementComponent.CameraMovementComponent_C|GetZoomSpeed (Variables|Default|GetMovementComponent))))))

(event EventBeginPlay
  (Transformation|SetWorldLocation (Variables|Collision|GetCapsuleComponent) "1200.000000,1200.000000,200.000000" false false)
  (Variables|/Script/Engine.SpringArmComponent|SetTargetArmLength (Variables|Default|GetSpringArm) 4e+03))

(fn ConstructionScript)